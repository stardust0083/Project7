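; Player character Blueprint for a shooter that manages the local HUD and supplies replicated state for animation.
; On BeginPlay the locally controlled player gets normal and sniper crosshairs plus a health bar; aiming with an "RF" gun swaps crosshairs.
; Each tick, owning client or authority pushes clamped aim pitch/yaw and jump, crouch and aim flags into character variables, working around non-replicating Animation Blueprint variables.
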(event Custom|SendYawPitch
  (params (Pitch :type Float%20%28single-precision%29) (Yaw :type Float%20%28single-precision%29))
  ;[1 1 1] Use replicated character variable to control animation (variable in animation blueprint doesn't work)
  (Variables|Default|SetPitchBP Pitch)
  (Variables|Default|SetYawBP Yaw))

(event Custom|SyncJumping
  ;[1 1 1] Use replicated character variable to control animation (variable in animation blueprint doesn't work)
  (bind _ascharacter (Utilities|Casting|CastToCharacter (Class|PawnMovementComponent|GetPawnOwner (Variables|Character|GetCharacterMovement))))
  (Variables|Default|SetIsJumping (Variables|/Script/Engine.Character|GetbWasJumping _ascharacter)))

(event Custom|SyncCrouching
  ;[1 1 1] Use replicated character variable to control animation (variable in animation blueprint doesn't work)
  (bind _ascharacter (Utilities|Casting|CastToCharacter (Class|PawnMovementComponent|GetPawnOwner (Variables|Character|GetCharacterMovement))))
  (Variables|Default|SetIsCrouching (Variables|/Script/Engine.Character|GetbIsCrouched _ascharacter)))

(event Custom|SyncAiming
  ;[1 1 1] Use replicated character variable to control animation (variable in animation blueprint doesn't work)
  (bind _astpscharacter (Utilities|Casting|CastToTPSCharacter (Class|PawnMovementComponent|GetPawnOwner (Variables|Character|GetCharacterMovement))))
  (Variables|Default|SetIsAiming (Variables|/Script/FinalProject.TPSCharacter|GetbAiming _astpscharacter)))

(event EventBeginPlay
  ;[1 1 1] Create UMG and add to viewport
  (if (Pawn|IsLocallyControlled)
    (bind _returnvalue (UserInterface|CreateWidget "/Game/UI/CrossAim.CrossAim_C"))
    (bind _output_get (Variables|Default|SetCrossAimOrdinary _returnvalue))
    (UserInterface|Viewport|AddtoViewport _output_get 0)
    (bind _returnvalue_2 (UserInterface|CreateWidget "/Game/UI/CrossAim_2.CrossAim_2_C"))
    (bind _output_get_2 (Variables|Default|SetCrossAimSniper _returnvalue_2))
    (UserInterface|Viewport|AddtoViewport _output_get_2 0)
    (Widget|SetVisibility _output_get_2 "Hidden")
    (bind _returnvalue_3 (UserInterface|CreateWidget "/Game/UI/HealthBar.HealthBar_C"))
    (UserInterface|Viewport|AddtoViewport _returnvalue_3 0)))

(event Collision|EventActorBeginOverlap
  (params (OtherActor :type Actor%20Object%20Reference)))

(event EventTick
  (params (DeltaSeconds :type Float%20%28single-precision%29))
  ;[1 1 1] Use replicated character variable to control animation (variable in animation blueprint doesn't work)
  (Utilities|FlowControl|Sequence
    (:then_0
      (if (or (Pawn|IsLocallyControlled) (Ability|HasAuthority))
        (Variables|Default|SetReplicatedRotation (Pawn|GetControlRotation :!class /Script/Engine.Pawn))))
    (:then_1
      (if (or (Utilities|Enum|Equal(Enum) (Networking|GetLocalRole) "ROLE_AutonomousProxy") (Ability|HasAuthority))
        (CallFunction|SendYawPitch (Math|Float|ClampAngle (.pitch (Math|Rotator|Delta(Rotator) (Variables|Default|GetReplicatedRotation) (Transformation|GetActorRotation))) -9e+01 9e+01) (Math|Float|ClampAngle (.yaw (Math|Rotator|Delta(Rotator) (Variables|Default|GetReplicatedRotation) (Transformation|GetActorRotation))) -9e+01 9e+01))
        (CallFunction|SyncJumping)
        (CallFunction|SyncCrouching)
        (CallFunction|SyncAiming)))))

(event Input|ActionEvents|InputActionAim
  (params (Key :type Key%20Structure))
  ;[1 1 1] Aiming UMG control
  (:Pressed
    (Class|TPSCharacter|BeginAiming)
    (Development|PrintString "Aiming")
    (if (Utilities|Name|Equal(Name) (Variables|/Script/FinalProject.TPSWeapon|GetGunType (Variables|Default|GetEquippedWeapon)) "RF")
      (Widget|SetVisibility (Variables|Default|GetCrossAimSniper) "Visible")
      (Widget|SetVisibility (Variables|Default|GetCrossAimOrdinary) "Hidden")))
  (:Released
    (Class|TPSCharacter|EndAiming)
    (Development|PrintString "AimingNot")
    (if (Utilities|Name|Equal(Name) (Variables|/Script/FinalProject.TPSWeapon|GetGunType (Variables|Default|GetEquippedWeapon)) "RF")
      (Widget|SetVisibility (Variables|Default|GetCrossAimSniper) "Hidden")
      (Widget|SetVisibility (Variables|Default|GetCrossAimOrdinary) "Visible"))))

(fn ConstructionScript)