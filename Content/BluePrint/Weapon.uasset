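; Weapon actor that configures itself on BeginPlay as one of five gun types: assault rifle, shotgun, grenade launcher, rocket launcher or sniper rifle.
; A switch on GunType's string value sets the skeletal mesh, fire effect and sound, impact effect, spread and fire interval.
; Only the rifles and shotgun set bullet and headshot damage; both launchers use explosion impact effects.
; Firing logic is absent here, and overlap and tick events are empty.
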(event EventBeginPlay
  (bind _weaponmeshcomponent (Variables|Default|GetWeaponMeshComponent))
  (switch string (Utilities|String|ToString(Name) (Variables|Default|GetGunType))
    (:AR
      (Class|SkinnedMeshComponent|SetSkeletalMesh _weaponmeshcomponent "/Game/MilitaryWeapSilver/Weapons/Assault_Rifle_A.Assault_Rifle_A" false)
      (Variables|Default|SetFireEffect "/Game/MilitaryWeapSilver/FX/P_AssaultRifle_MuzzleFlash.P_AssaultRifle_MuzzleFlash")
      (Variables|Default|SetFireSound "/Game/MilitaryWeapSilver/Sound/Rifle/Wavs/RifleA_Fire02.RifleA_Fire02")
      (Variables|Default|SetImpactEffect "/Game/MilitaryWeapSilver/FX/P_Impact_Metal_Medium_01.P_Impact_Metal_Medium_01")
      (Variables|Default|SetBulletTraceSpread 3.0)
      (Variables|Default|SetFireGapTime 0.0)
      (Variables|Default|SetBulletDamage 2e+01)
      (Variables|Default|SetHeadShotDamage 4e+01))
    (:SG
      (Class|SkinnedMeshComponent|SetSkeletalMesh _weaponmeshcomponent "/Game/MilitaryWeapSilver/Weapons/Shotgun_A.Shotgun_A" false)
      (Variables|Default|SetFireEffect "/Game/MilitaryWeapSilver/FX/P_Shotgun_MuzzleFlash_01.P_Shotgun_MuzzleFlash_01")
      (Variables|Default|SetFireSound "/Game/MilitaryWeapSilver/Sound/Shotgun/Wavs/ShotgunA_Fire01.ShotgunA_Fire01")
      (Variables|Default|SetImpactEffect "/Game/MilitaryWeapSilver/FX/P_Impact_Metal_Medium_01.P_Impact_Metal_Medium_01")
      (Variables|Default|SetBulletTraceSpread 1e+01)
      (Variables|Default|SetFireGapTime 1.0)
      (Variables|Default|SetBulletDamage 1e+01)
      (Variables|Default|SetHeadShotDamage 2e+01))
    (:GL
      (Class|SkinnedMeshComponent|SetSkeletalMesh _weaponmeshcomponent "/Game/MilitaryWeapSilver/Weapons/Grenade_Launcher_A.Grenade_Launcher_A" false)
      (Variables|Default|SetFireEffect "/Game/MilitaryWeapSilver/FX/P_Grenade_MuzzleFlash_01.P_Grenade_MuzzleFlash_01")
      (Variables|Default|SetFireSound "/Game/MilitaryWeapSilver/Sound/GrenadeLauncher/Wavs/GrenadeLauncherA_Fire01.GrenadeLauncherA_Fire01")
      (Variables|Default|SetImpactEffect "/Game/MilitaryWeapSilver/FX/P_Grenade_Explosion_01.P_Grenade_Explosion_01")
      (Variables|Default|SetBulletTraceSpread 0.0)
      (Variables|Default|SetFireGapTime 0.5))
    (:RL
      (Class|SkinnedMeshComponent|SetSkeletalMesh _weaponmeshcomponent "/Game/MilitaryWeapSilver/Weapons/Rocket_Launcher_A.Rocket_Launcher_A" false)
      (Variables|Default|SetFireEffect "/Game/MilitaryWeapSilver/FX/P_RocketLauncher_MuzzleFlash_Front_01.P_RocketLauncher_MuzzleFlash_Front_01")
      (Variables|Default|SetFireSound "/Game/MilitaryWeapSilver/Sound/RocketLauncher/Wavs/RocketLauncherA_Fire01.RocketLauncherA_Fire01")
      (Variables|Default|SetImpactEffect "/Game/MilitaryWeapSilver/FX/P_RocketLauncher_Explosion_01.P_RocketLauncher_Explosion_01")
      (Variables|Default|SetBulletTraceSpread 0.0)
      (Variables|Default|SetFireGapTime 2.0))
    (:RF
      (Class|SkinnedMeshComponent|SetSkeletalMesh _weaponmeshcomponent "/Game/MilitaryWeapSilver/Weapons/Sniper_Rifle_A.Sniper_Rifle_A" false)
      (Variables|Default|SetFireEffect "/Game/MilitaryWeapSilver/FX/P_SniperRifle_MuzzleFlash_01.P_SniperRifle_MuzzleFlash_01")
      (Variables|Default|SetFireSound "/Game/MilitaryWeapSilver/Sound/SniperRifle/Wavs/SniperRifleA_Fire01.SniperRifleA_Fire01")
      (Variables|Default|SetImpactEffect "/Game/MilitaryWeapSilver/FX/P_Impact_Metal_Large_01.P_Impact_Metal_Large_01")
      (Variables|Default|SetBulletTraceSpread 0.0)
      (Variables|Default|SetFireGapTime 1.0)
      (Variables|Default|SetBulletDamage 5e+01)
      (Variables|Default|SetHeadShotDamage 2e+02))))

(event Collision|EventActorBeginOverlap
  (params (OtherActor :type Actor%20Object%20Reference)))

(event EventTick
  (params (DeltaSeconds :type Float%20%28single-precision%29)))

(fn ConstructionScript)