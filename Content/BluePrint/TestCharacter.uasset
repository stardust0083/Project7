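; TestCharacter is a character Blueprint that sets up crosshair widgets for weapon aiming.
; BeginPlay creates and adds an ordinary and a sniper crosshair to the viewport, with the sniper one hidden.
; Unconnected BeginAiming and EndAiming chains would swap crosshair visibility for "RF" GunType weapons but never run, as does a stray FireTest call.
; Overlap and Tick events are disabled stubs, and the construction script is empty.
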(event EventBeginPlay
  (bind _returnvalue (UserInterface|CreateWidget "/Game/UI/CrossAim.CrossAim_C"))
  (bind _output_get (Variables|Default|SetCrossAimOrdinary _returnvalue))
  (UserInterface|Viewport|AddtoViewport _output_get 0)
  (bind _returnvalue_2 (UserInterface|CreateWidget "/Game/UI/CrossAim_2.CrossAim_2_C"))
  (bind _output_get_2 (Variables|Default|SetCrossAimSniper _returnvalue_2))
  (UserInterface|Viewport|AddtoViewport _output_get_2 0)
  (Widget|SetVisibility _output_get_2 "Hidden"))

(event Collision|EventActorBeginOverlap
  (params (OtherActor :type Actor%20Object%20Reference)))

(event EventTick
  (params (DeltaSeconds :type Float%20%28single-precision%29)))

(event Input|ActionEvents|InputActionAim
  (params (Key :type Key%20Structure :default "None")))

(event Input|MouseEvents|LeftMouseButton
  (params (Key :type Key%20Structure :default "None")))

(fn ConstructionScript)